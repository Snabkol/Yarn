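; PlayerHUD is an actor component that shows the player's health and resource levels on screen.
; On BeginPlay it creates WBP_PlayerHUD, adds it to the viewport and caches the player character as BP_Avatar.
; UpdateHealth and UpdateResource set bar percentages from the avatar's EntityStats when called, with no polling or binding here.
; UpdateResource switches on ResourceType, filling the resource bar for Mana or Energy and the health bar for Health.
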(event `self.ReceiveBeginPlay`
  (bind _returnvalue (`|CreateWidget` "/Game/Custom/UI/WBP_PlayerHUD.WBP_PlayerHUD_C"))
  (set `self.Widget Reference` _returnvalue)
  (`UserWidget.AddToViewport` _returnvalue 0)
  (bind _asbp_avatar (cast `/Game/Custom/Blueprints/BP_Avatar` (`GameplayStatics.GetPlayerCharacter` 0)))
  (set `self.AvatarReference` _asbp_avatar))

(fn `UpdateHealth`
  (bind _entitystats (`/Game/Custom/Blueprints/BP_Avatar.EntityStats` (`self.AvatarReference`)))
  (`ProgressBar.SetPercent` (`/Game/Custom/UI/WBP_PlayerHUD.HealthBar` (`self.Widget Reference`)) (/ (`/Game/Custom/Blueprints/ActorComponents/EntityStats.Current Health` _entitystats) (`/Game/Custom/Blueprints/ActorComponents/EntityStats.Max Health` _entitystats))))

(fn `UpdateResource`
  (bind _entitystats (`/Game/Custom/Blueprints/BP_Avatar.EntityStats` (`self.AvatarReference`)))
  (bind _entitystats_2 (`/Game/Custom/Blueprints/BP_Avatar.EntityStats` (`self.AvatarReference`)))
  (bind _entitystats_3 (`/Game/Custom/Blueprints/BP_Avatar.EntityStats` (`self.AvatarReference`)))
  (switch `/Game/Custom/Blueprints/AbilitySystem/E_ResourceType` (`/Game/Custom/Blueprints/ActorComponents/EntityStats.ResourceType` (`/Game/Custom/Blueprints/BP_Avatar.EntityStats` (`self.AvatarReference`)))
    (:`NewEnumerator1`
      (`ProgressBar.SetPercent` (`/Game/Custom/UI/WBP_PlayerHUD.ResourceBar` (`self.Widget Reference`)) (`KismetMathLibrary.Conv_IntToDouble` (/ (`/Game/Custom/Blueprints/ActorComponents/EntityStats.Current Mana` _entitystats_2) (`/Game/Custom/Blueprints/ActorComponents/EntityStats.Max Mana` _entitystats_2)))))
    (:`NewEnumerator2`
      (`ProgressBar.SetPercent` (`/Game/Custom/UI/WBP_PlayerHUD.ResourceBar` (`self.Widget Reference`)) (`KismetMathLibrary.Conv_IntToDouble` (/ (`/Game/Custom/Blueprints/ActorComponents/EntityStats.Current Energy` _entitystats) (`/Game/Custom/Blueprints/ActorComponents/EntityStats.Max Energy` _entitystats)))))
    (:`NewEnumerator0`
      (`ProgressBar.SetPercent` (`/Game/Custom/UI/WBP_PlayerHUD.HealthBar` (`self.Widget Reference`)) (`KismetMathLibrary.SafeDivide` (`/Game/Custom/Blueprints/ActorComponents/EntityStats.Current Health` _entitystats_3) (`/Game/Custom/Blueprints/ActorComponents/EntityStats.Max Health` _entitystats_3))))))