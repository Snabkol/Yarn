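; BP_Avatar is a top-down character that emits movement noise others can hear and can probe obstacles for vaulting.
; A looping timer sets the sound mode from falling, crouching, running or walking; MakeSound then sphere-traces that mode's radius and notifies IF_Hearing actors.
; VaultMotionWarp traces forward, then downward, to store vault start, middle and landing positions, without applying a warp here.
; SetHoveredActor also runs on a timer but is empty.
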(event `self.ReceiveBeginPlay`
  (`KismetSystemLibrary.K2_SetTimer` null "SetHoveredActor" 0.01 true)
  (`KismetSystemLibrary.K2_SetTimer` null "SetSoundMode" 0.01 true))

(fn `MakeSound`
  (locals (NoiseDebug :type "EDrawDebugTrace Enum" :default "ForOneFrame"))
  (bind _returnvalue (`self.K2_GetActorLocation`))
  (if (>= (`KismetMathLibrary.VSize` (`MovementComponent.Velocity` (`self.CharacterMovement`))) 50.0)
    (bind (_outhits _returnvalue_2) (`KismetSystemLibrary.SphereTraceMulti` _returnvalue _returnvalue (`BlueprintMapLibrary.Map_Find` (`self.MovementSoundModeMap`) (`self.CurrentSoundMode`)) "TraceTypeQuery1"))
    (if _returnvalue_2
      (for _array_element _outhits
        (bind (_bblockinghit _binitialoverlap _time _distance _location _impactpoint _normal _impactnormal _physmat _hitactor _hitcomponent _hitbonename _bonename _hititem _elementindex _faceindex _tracestart) (`GameplayStatics.BreakHitResult` _array_element))
        (if (`KismetSystemLibrary.DoesImplementInterface` _hitactor "/Game/Custom/Blueprints/Interfaces/IF_Hearing.IF_Hearing_C")
          (message `/Game/Custom/Blueprints/Interfaces/IF_Hearing.HeardNoise` _hitactor _tracestart self))))))

(fn `SetHoveredActor`)

(fn `SetSoundMode`
  (if (`NavMovementComponent.IsFalling` (`self.CharacterMovement`))
    (set `self.CurrentSoundMode` "NewEnumerator0")
    (`self.MakeSound` :!label _label)
    (elif (`NavMovementComponent.IsCrouching` (`self.CharacterMovement`))
      (set `self.CurrentSoundMode` "NewEnumerator2")
      (goto _label)
      (elif (`/Game/Custom/Blueprints/BP_TopDownController.Running` (cast `/Game/Custom/Blueprints/BP_TopDownController` (`self.GetController`) :!pure true))
        (set `self.CurrentSoundMode` "NewEnumerator3")
        (goto _label)
        (elif (`CharacterMovementComponent.IsWalking` (`self.CharacterMovement`))
          (set `self.CurrentSoundMode` "NewEnumerator1")
          (goto _label))))))

(fn `UserConstructionScript`)

(fn `VaultMotionWarp`
  (for _index (range 3)
    (bind _returnvalue (+ (`self.K2_GetActorLocation`) (`KismetMathLibrary.MakeVector` 0.0 0.0 (* _index 30))))
    (bind (_outhit _returnvalue_2) (`KismetSystemLibrary.SphereTraceSingle` :`Start` _returnvalue :`End` (+ _returnvalue (* (`self.GetActorForwardVector`) 180.0)) :`Radius` 5.0 :`TraceChannel` "TraceTypeQuery1" :`DrawDebugType` (`self.VaultTraceDrawType`) :`DrawTime` (`self.VaultTraceDrawTime`)))
    (if _returnvalue_2
      (`|ExecutionSequence`
        (:`then_0`
          (break))
        (:`then_1`
          (for _index_2 (range 6)
            (bind _returnvalue_3 (+ (+ (`.Location` (`GameplayStatics.BreakHitResult` _outhit)) (0.0 0.0 100.0)) (* (`self.GetActorForwardVector`) (* _index_2 50))))
            (bind (_outhit_2 _returnvalue_4) (`KismetSystemLibrary.SphereTraceSingle` :`Start` _returnvalue_3 :`End` (- _returnvalue_3 (0.0 0.0 100.0)) :`Radius` 5.0 :`TraceChannel` "TraceTypeQuery1" :`DrawDebugType` (`self.VaultTraceDrawType`) :`DrawTime` (`self.VaultTraceDrawTime`)))
            (if _returnvalue_4
              (`|ExecutionSequence`
                (:`then_0`
                  (if (== _index_2 0)
                    (bind (_bblockinghit _binitialoverlap _time _distance _location _impactpoint _normal _impactnormal _physmat _hitactor _hitcomponent _hitbonename _bonename _hititem _elementindex _faceindex _tracestart) (`GameplayStatics.BreakHitResult` _outhit_2))
                    (bind _output_get (set `self.VaultStartPosition` _location))
                    (`KismetSystemLibrary.DrawDebugSphere` _output_get 10.0 12 (struct :`R` 1.0 :`G` 1.0 :`B` 1.0 :`A` 1.0) (`self.VaultTraceDrawTime`))))
                (:`then_1`
                  (bind _output_get_2 (set `self.VaultMiddlePosition` _location))
                  (`KismetSystemLibrary.DrawDebugSphere` _output_get_2 10.0 12 (struct :`R` 1.0 :`B` 0.909885 :`A` 1.0) (`self.VaultTraceDrawTime`))))
              (else
                (bind _returnvalue_5 (+ _tracestart (* (`self.GetActorForwardVector`) (`self.VaultLandingOffset`))))
                (bind (_outhit_3 _returnvalue_6) (`KismetSystemLibrary.LineTraceSingle` :`Start` _returnvalue_5 :`End` (- _returnvalue_5 (0.0 0.0 1000.0)) :`TraceChannel` "TraceTypeQuery1" :`DrawDebugType` (`self.VaultTraceDrawType`) :`TraceColor` (struct :`B` 1.0 :`A` 1.0) :`DrawTime` (`self.VaultTraceDrawTime`))) ; Vault Landing Position
                (if _returnvalue_6
                  (set `self.VaultLandingPosition` (`.Location` (`GameplayStatics.BreakHitResult` _outhit_3)))
                  (break))))))))))