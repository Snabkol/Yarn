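; BP_Door is an interactable door that swings open and shut by 90 degrees of yaw on alternate activations.
; Interact requires the player in range and, when locked, a matching key name in BP_Avatar's CollectedKeys; ButtonInteract bypasses both checks.
; On BeginPlay it stores its starting yaw and passes its KeyName to any referenced key.
; A FlipFlop drives the DoorState timeline and Tampered flag, with mesh collision disabled during the swing.
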(event `self.ReceiveBeginPlay`
  (bind (_returnvalue_roll _returnvalue_pitch _returnvalue_yaw) (`KismetMathLibrary.BreakRotator` (`self.K2_GetActorRotation`)))
  (`parent.ReceiveBeginPlay`)
  (set `self.StartRotation` _returnvalue_yaw)
  (bind _key_reference (`self.Key Reference`)
    (:`then`
      (set `/Game/Custom/Blueprints/Interactable/BP_Key.KeyName` (`self.KeyName`) _key_reference))
    (:`else`)))

(event `/Game/Custom/Blueprints/Interfaces/IF_Interactable.ButtonInteract`
  (bind _startrotation (`self.StartRotation`))
  (`PrimitiveComponent.SetCollisionEnabled` (`self.Mesh`) "NoCollision" :!label _label)
  (`/Engine/EditorBlueprintResources/StandardMacros.FlipFlop`
    (:`A`
      (set `self.Tampered` true)
      (bind (_direction _alpha) (`Timeline|DoorState` :!label _label_2)
        (:`Update`
          (`self.K2_SetActorRotation` (`KismetMathLibrary.MakeRotator` 0.0 0.0 (`|EaseFunction` "Linear" _alpha _startrotation (+ _startrotation 90.0)))) ; Rotate in Yaw
        )
        (:`Finished`
          (`PrimitiveComponent.SetCollisionEnabled` (`self.Mesh`) "QueryAndPhysics"))))
    (:`B`
      (set `self.Tampered` false)
      (goto _label_2 :!via `Reverse`))))

(event `/Game/Custom/Blueprints/Interfaces/IF_Interactable.Interact`
  (params (Avatar :type "/Game/Custom/Blueprints/BP_Avatar Object Reference"))
  (if (`/Game/Custom/Blueprints/Interactable/AC_InteractRange.PlayerInRange` (`self.Interact Range`))
    (if (`self.Locked`)
      (bind _asbp_avatar (cast `/Game/Custom/Blueprints/BP_Avatar` (`GameplayStatics.GetPlayerCharacter` 0)))
      (if (`BlueprintSetLibrary.Set_Contains` (`/Game/Custom/Blueprints/BP_Avatar.CollectedKeys` _asbp_avatar) (`self.KeyName`))
        (goto _label))
      (else
        (goto _label)))))

(fn `UserConstructionScript`)