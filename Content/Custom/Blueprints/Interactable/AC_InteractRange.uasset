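; AC_InteractRange is a component that tracks whether the player avatar is within interaction range of its owning actor.
; Each tick it runs a zero-length sphere trace for Pawn objects at the owner's location, using InteractRange as radius and DrawRange for debug drawing.
; PlayerInRange is true only when the single returned hit's class is exactly BP_Avatar, so subclasses or another pawn being hit leave it false.
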(event `self.ReceiveTick`
  (params (DeltaSeconds :type "Float (single-precision)"))
  (bind _returnvalue (`Actor.K2_GetActorLocation` (`self.GetOwner`)))
  (bind (_outhit _returnvalue_2) (`KismetSystemLibrary.SphereTraceSingleForObjects` :`Start` _returnvalue :`End` _returnvalue :`Radius` (`self.InteractRange`) :`ObjectTypes` (`|MakeArray` "ObjectTypeQuery3" :!type "EObjectTypeQuery Enum") :`DrawDebugType` (`self.DrawRange`)))
  (if _returnvalue_2
    (if (== (`GameplayStatics.GetObjectClass` (`.HitActor` (`GameplayStatics.BreakHitResult` _outhit))) "/Game/Custom/Blueprints/BP_Avatar.BP_Avatar_C")
      (set `self.PlayerInRange` true)
      (else
        (set `self.PlayerInRange` false)))
    (else
      (set `self.PlayerInRange` false))))