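; BP_InteractBase is an interactable actor base that shows a prompt and flags its meshes for highlighting on cursor hover.
; BeginPlay creates a WBP_InteractWidget from InteractText and assigns it to the InteractWidget component.
; Hover reveals the prompt and enables custom depth on static meshes if InteractRange reports the player in range, otherwise retrying on a short timer.
; Cursor exit cancels the retry, hides the prompt and disables custom depth.
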(event `self.ReceiveBeginPlay`
  (bind _returnvalue (`|CreateWidget` "/Game/Custom/UI/WBP_InteractWidget.WBP_InteractWidget_C" null (`self.InteractText`)))
  (`WidgetComponent.SetWidget` (`self.InteractWidget`) _returnvalue))

(event `self.ReceiveActorBeginCursorOver`
  (if (`/Game/Custom/Blueprints/Interactable/AC_InteractRange.PlayerInRange` (`self.Interact Range`)) :!label _label
    (`SceneComponent.SetHiddenInGame` (`self.InteractWidget`) false false)
    (for _array_element (`self.K2_GetComponentsByClass` "/Script/Engine.StaticMeshComponent")
      (`PrimitiveComponent.SetRenderCustomDepth` _array_element true))
    (else
      (bind _returnvalue (`KismetSystemLibrary.K2_SetTimerDelegate` (delegate `RetryCursorHighlight`) 0.1))
      (set `self.RetryCursorHighlightTimer` _returnvalue))))

(event `RetryCursorHighlight`
  (goto _label))

(event `self.ReceiveActorEndCursorOver`
  (`KismetSystemLibrary.K2_ClearAndInvalidateTimerHandle` (`self.RetryCursorHighlightTimer`))
  (`SceneComponent.SetHiddenInGame` (`self.InteractWidget`) true false)
  (for _array_element (`self.K2_GetComponentsByClass` "/Script/Engine.StaticMeshComponent")
    (`PrimitiveComponent.SetRenderCustomDepth` _array_element false)))

(fn `UserConstructionScript`)