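; BP_Button is a one-shot interactable push button that triggers a referenced interactable.
; On first interaction, a ButtonPush timeline lowers the mesh from its cached starting position.
; When the press finishes, it calls ButtonInteract on the reference, turns the mesh material green and reverses the timeline to raise the button.
; A pushed flag blocks repeat presses and suppresses the parent's cursor-over behavior.
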(event `self.ReceiveBeginPlay`
  (`parent.ReceiveBeginPlay`)
  (set `self.Relative Location` (`SceneComponent.RelativeLocation` (`self.Mesh`))))

(event `self.Interact`
  (params (Avatar :type "/Game/Custom/Blueprints/BP_Avatar Object Reference"))
  (if (not (`self.HasBeenPushed`))
    (set `self.HasBeenPushed` true)
    (bind (_direction _alpha) (`Timeline|ButtonPush` :!label _label)
      (:`Update`
        (`SceneComponent.K2_SetRelativeLocation` (`self.Mesh`) (`KismetMathLibrary.VLerp` (`self.Relative Location`) (- (`self.Relative Location`) (0.0 0.0 4.5)) _alpha) false false))
      (:`Finished`
        (if (`|EnumEquality` _direction "Forward")
          (`self.ButtonInteract` (`self.InteractableReference`))
          (`PrimitiveComponent.SetMaterial` (`self.Mesh`) 0 "/Game/Custom/Materials/MI_Green.MI_Green")
          (`self.ReturnButton`))))))

(event `ReturnButton`
  (goto _label :!via `Reverse`))

(event `self.ReceiveActorBeginCursorOver`
  (if (not (`self.HasBeenPushed`))
    (`parent.ReceiveActorBeginCursorOver`)))

(fn `UserConstructionScript`
  (`parent.UserConstructionScript`))