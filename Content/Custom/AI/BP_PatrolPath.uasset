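; BP_PatrolPath is a patrol waypoint that moves BP_Dummy AI along its patrol route.
; A Sphere overlap starts a PatrolChangeDelay wait, then casts the overlapping actor to BP_Dummy.
; If this waypoint is in that dummy's PatrolPoints, it increments CurrentPatrolIndex, wrapping to zero past the last point.
; The Delay precedes the cast, so any overlapping actor starts the shared timer.
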(event `self.Sphere.OnComponentBeginOverlap`
  (params (OverlappedComponent :type "PrimitiveComponent Object Reference") (OtherActor :type "Actor Object Reference") (OtherComp :type "PrimitiveComponent Object Reference") (OtherBodyIndex :type Integer) (bFromSweep :type Boolean) (SweepResult :type "HitResult Structure (by ref)"))
  (`KismetSystemLibrary.Delay` (`self.PatrolChangeDelay`))
  (bind _asbp_dummy (cast `/Game/Custom/Blueprints/BP_Dummy` OtherActor))
  (bind _patrolpoints (`/Game/Custom/Blueprints/BP_Dummy.PatrolPoints` _asbp_dummy))
  (if (`KismetArrayLibrary.Array_Contains` _patrolpoints self)
    (bind _result (`/Engine/EditorBlueprintResources/StandardMacros.IncrementInt` (`/Game/Custom/Blueprints/BP_Dummy.CurrentPatrolIndex` _asbp_dummy))
      (:`  `
        (if (> _result (- (`KismetArrayLibrary.Array_Length` _patrolpoints) 1))
          (set `/Game/Custom/Blueprints/BP_Dummy.CurrentPatrolIndex` 0 _asbp_dummy))))))

(fn `UserConstructionScript`)